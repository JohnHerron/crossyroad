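; Moving log actor, driven by a ProjectileMovement component, that randomizes its size and speed when spawned.
; On BeginPlay a three-way random roll picks the large mesh, the small mesh, or leaves the default mesh and speeds untouched.
; The large and small variants each roll InitialSpeed and MaxSpeed separately within their own range, so the two values can differ.
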(event EventBeginPlay
  (bind _returnvalue (Math|Random|RandomIntegerinRange 70 100))
  (bind _returnvalue_2 (Math|Random|RandomIntegerinRange 60 100))
  (bind _projectilemovement (Variables|Default|GetProjectileMovement))
  (bind _projectilemovement_2 (Variables|Default|GetProjectileMovement))
  (switch int (Math|Random|RandomIntegerinRange 0 2)
    (:1
      (Variables|/Script/Engine.ProjectileMovementComponent|SetInitialSpeed _projectilemovement_2 (Math|Conversions|ToFloat(Integer) _returnvalue_2))
      (Variables|/Script/Engine.ProjectileMovementComponent|SetMaxSpeed _projectilemovement_2 (Math|Conversions|ToFloat(Integer) _returnvalue_2))
      (Components|StaticMesh|SetStaticMesh (Variables|Default|Getlog) "/Game/StarterContent/River/log_large.log_large"))
    (:2
      (Variables|/Script/Engine.ProjectileMovementComponent|SetInitialSpeed _projectilemovement (Math|Conversions|ToFloat(Integer) _returnvalue))
      (Variables|/Script/Engine.ProjectileMovementComponent|SetMaxSpeed _projectilemovement (Math|Conversions|ToFloat(Integer) _returnvalue))
      (Components|StaticMesh|SetStaticMesh (Variables|Default|Getlog) "/Game/StarterContent/River/log_small.log_small"))))

(fn ConstructionScript)