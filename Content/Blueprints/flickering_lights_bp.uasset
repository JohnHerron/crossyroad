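; Flickering lights Blueprint that alternates two point lights, so one is lit while the other is dark.
; Tick accumulates delta time and calls SwitchLights each time the total exceeds one second, then resets the counter.
; SwitchLights uses the CurrLight boolean as a toggle, swapping the two lights' intensities between off and full on a fixed, non-random rhythm.
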(event EventTick
  (params (DeltaSeconds :type Float%20%28single-precision%29))
  (bind _output_get (Variables|Default|Settime_since_last_flicker (+ DeltaSeconds (Variables|Default|Gettime_since_last_flicker) 0.0)))
  (Math|Float|CompareFloat _output_get 1.0
    (:>
      (CallFunction|SwitchLights)
      (Variables|Default|Settime_since_last_flicker 0.0))))

(fn ConstructionScript)

(fn SwitchLights
  (if (Variables|Default|GetcurrLight)
    (Rendering|Components|Light|SetIntensity (Variables|Default|GetPointLight) 0.0)
    (Rendering|Components|Light|SetIntensity (Variables|Default|GetPointLight1) 5e+03)
    (Variables|Default|SetcurrLight false)
    (else
      (Rendering|Components|Light|SetIntensity (Variables|Default|GetPointLight) 5e+03)
      (Rendering|Components|Light|SetIntensity (Variables|Default|GetPointLight1) 0.0)
      (Variables|Default|SetcurrLight true))))