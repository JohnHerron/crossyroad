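; Lane spawner that builds a chained strip of grass, water and railroad lanes, apparently for a Crossy Road-style endless level.
; BeginPlay clears existing lanes and spawns an initial batch from near the player, each attaching at the previous lane's SpawnPoint.
; Lane types come in runs of random length, starting with bright grass.
; Each spawn gives the lane a spawner reference and destroys tracked lanes far behind the player on X.
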(event EventBeginPlay
  (Variables|Default|SetNumOfCurrentLanes 10)
  (Variables|Default|SetCurrent%20Lane%20Type "/Game/StarterContent/Other/brightgrass.brightgrass")
  (CallFunction|SpawnInitialLanes))

(fn ConstructionScript)

(fn SpawnLaneatSpawnPoint
  (CallFunction|SpawnLane (Transformation|GetWorldLocation (Variables|/Game/Blueprints/lane_bp.lane_bp_C|GetSpawnPoint (Variables|Default|GetNewestLane)))))

(fn SpawnLane
  (params (Location :type Vector))
  (bind _returnvalue (Game|SpawnActorfromClass "/Game/Blueprints/lane_bp.lane_bp_C" (Math|Transform|MakeTransform Location "0, 0, 0" "1,1,1") "Undefined" 0 0))
  (bind _output_get (Variables|Default|SetNewestLane _returnvalue))
  (bind _output_get_2 (Variables|/Game/Blueprints/lane_bp.lane_bp_C|SetLaneSpawner _output_get self))
  (CallFunction|ChooseLaneType _output_get_2 _output_get)
  (CallFunction|DestroyFarLanes))

(fn SpawnInitialLanes
  (Utilities|FlowControl|Sequence
    (:then_0
      (bind _outactors (Actor|GetAllActorsOfClass "/Game/Blueprints/lane_bp.lane_bp_C"))
      (for _array_element _outactors
        (Actor|DestroyActor _array_element)))
    (:then_1
      (for _index (range 0 20)
        (Utilities|IsValid (Variables|Default|GetNewestLane)
          (:Is%20Valid
            (CallFunction|SpawnLaneatSpawnPoint))
          (:Is%20Not%20Valid
            (CallFunction|SpawnLane (+ (Transformation|GetActorLocation (Game|Player|GetPlayerPawn 0)) "-500.000000,-750.000000,-50.000000"))))))))

(fn ChooseLaneType
  (params (NewestLane :type Lane%20Bp%20Object%20Reference))
  (bind _numofcurrentlanes (Variables|Default|GetNumOfCurrentLanes))
  (if (!= _numofcurrentlanes 0)
    (Math|Integer|DecrementInt _numofcurrentlanes
      (:%20%20
        _))
    (else
      (CallFunction|ChooseNumLanes)
      (CallFunction|ChooseType)))
  (Default|SetType (Variables|Default|GetNewestLane) (Variables|Default|GetCurrent%20Lane%20Type)))

(fn ChooseNumLanes
  (Variables|Default|SetNumOfCurrentLanes (+ (Math|Random|RandomInteger (Variables|Default|GetMaxLanesToSpawn)) 1)))

(fn ChooseType
  (Variables|Default|SetCurrent%20Lane%20Type (Utilities|Select :Index (Math|Random|RandomIntegerinRange 0 3) :Option%200 "/Game/StarterContent/Other/brightgrass.brightgrass" :Option%201 "/Game/StarterContent/River/waterbrightBase.waterbrightBase" :Option%202 "/Game/StarterContent/Other/railroad.railroad" :Option%203 "/Game/StarterContent/Other/darkgrass.darkgrass")))

(fn DestroyFarLanes
  (bind _lanearray (Variables|Default|GetLaneArray))
  (Utilities|Array|Add _lanearray (Variables|Default|GetNewestLane))
  (for _array_element _lanearray
    (Utilities|IsValid _array_element
      (:Is%20Valid
        (bind _output_get (Variables|Default|SettempLane _array_element))
        (Math|Float|CompareFloat (.x (- (Transformation|GetActorLocation (Game|Player|GetPlayerPawn 0)) (Transformation|GetWorldLocation (Variables|/Game/Blueprints/lane_bp.lane_bp_C|GetDespawnAnchor (Variables|Default|GettempLane))))) 1e+03
          (:>
            (Utilities|Array|RemoveItem (Variables|Default|GetLaneArray) _output_get)
            (Actor|DestroyActor _output_get)))))))