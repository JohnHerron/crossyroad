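; Vehicle actor, in a file named vehicle_spawner, that randomizes its look and speed on BeginPlay and moves through a ProjectileMovement component.
; A random integer from 0 to 3 selects a taxi, USPS truck or SUV mesh with matching movement speeds, rotating the truck and SUV meshes.
; A roll of 0 keeps the component defaults.
; It spawns no actors, and its construction script and CarArray function are empty.
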(event EventBeginPlay
  (bind _projectilemovement (Variables|Default|GetProjectileMovement))
  (bind _projectilemovement_2 (Variables|Default|GetProjectileMovement))
  (bind _projectilemovement_3 (Variables|Default|GetProjectileMovement))
  ;[1 1 1] Setting mesh and speeds
  (switch int (Math|Random|RandomIntegerinRange 0 3)
    (:1
      (Variables|/Script/Engine.ProjectileMovementComponent|SetInitialSpeed _projectilemovement_3 2e+02)
      (Variables|/Script/Engine.ProjectileMovementComponent|SetMaxSpeed _projectilemovement_3 2e+02)
      (Components|StaticMesh|SetStaticMesh (Variables|Default|Getcar) "/Game/StarterContent/Vehicles/taxi.taxi"))
    (:2
      (Variables|/Script/Engine.ProjectileMovementComponent|SetInitialSpeed _projectilemovement 2e+02)
      (Variables|/Script/Engine.ProjectileMovementComponent|SetMaxSpeed _projectilemovement 2e+02)
      (Components|StaticMesh|SetStaticMesh (Variables|Default|Getcar) "/Game/StarterContent/Vehicles/USPStruck.USPStruck")
      (Transformation|AddRelativeRotation (Variables|Default|Getcar) "0.000000,90.000000, 0" false false))
    (:3
      (Variables|/Script/Engine.ProjectileMovementComponent|SetInitialSpeed _projectilemovement_2 3e+02)
      (Variables|/Script/Engine.ProjectileMovementComponent|SetMaxSpeed _projectilemovement_2 3e+02)
      (Components|StaticMesh|SetStaticMesh (Variables|Default|Getcar) "/Game/StarterContent/Vehicles/suv.suv")
      (Transformation|AddRelativeRotation (Variables|Default|Getcar) "0.000000,90.000000, 0" false false))))

(fn ConstructionScript)

(fn CarArray)