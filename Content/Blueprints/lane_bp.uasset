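; Lane actor built from a row of static mesh tiles, which asks the LaneSpawner for another lane when the ThirdPersonCharacter overlaps its trigger.
; SetType dresses the tiles by terrain: uniform grass or railroad, water with distinct edge tiles, or highway.
; Grass flips shade through a flag kept on the LaneSpawner.
; The spawner's lane counters decide whether highway is plain or alternates marked and unmarked tiles.
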(event OnComponentBeginOverlap(TriggerZone)
  (params (OverlappedComponent :type Primitive%20Component%20Object%20Reference) (OtherActor :type Actor%20Object%20Reference) (OtherComp :type Primitive%20Component%20Object%20Reference) (OtherBodyIndex :type Integer) (bFromSweep :type Boolean) (SweepResult :type Hit%20Result%20Structure%20%28by%20ref%29))
  ;[1 1 1] Spawn Next Lane
  (Utilities|Casting|CastToThirdPersonCharacter OtherActor)
  (Default|SpawnLaneatSpawnPoint (Variables|Default|GetLaneSpawner)))

(fn ConstructionScript)

(fn SetType
  (params (MeshType :type Static%20Mesh%20Object%20Reference))
  (bind _lanespawner (Variables|Default|GetLaneSpawner))
  (bind _lanespawner_2 (Variables|Default|GetLaneSpawner))
  (bind _output_get (LocalVariables|SetcurrMesh MeshType))
  ;[1 1 1] Determine if grass
  (if (or (== _output_get "/Game/StarterContent/Other/darkgrass.darkgrass") (== _output_get "/Game/StarterContent/Other/brightgrass.brightgrass"))
    ;[1 1 1] Alternate grass type
    (bind _output_get_2 (Variables|/Game/Blueprints/lane_spawner_bp.lane_spawner_bp_C|SetgrassType _lanespawner (not (Variables|/Game/Blueprints/lane_spawner_bp.lane_spawner_bp_C|GetgrassType _lanespawner))))
    (if _output_get_2
      (LocalVariables|SetcurrMesh "/Game/StarterContent/Other/brightgrass.brightgrass")
      (else
        (LocalVariables|SetcurrMesh "/Game/StarterContent/Other/darkgrass.darkgrass")))
    ;[1 1 1] Set whole lane as one texture
    (Components|StaticMesh|SetStaticMesh (Variables|Default|GetStaticMesh) (LocalVariables|GetcurrMesh) :!label _label)
    (Components|StaticMesh|SetStaticMesh (Variables|Default|GetStaticMesh1) (LocalVariables|GetcurrMesh))
    (Components|StaticMesh|SetStaticMesh (Variables|Default|GetStaticMesh2) (LocalVariables|GetcurrMesh))
    (Components|StaticMesh|SetStaticMesh (Variables|Default|GetStaticMesh9) (LocalVariables|GetcurrMesh))
    (Components|StaticMesh|SetStaticMesh (Variables|Default|GetStaticMesh4) (LocalVariables|GetcurrMesh))
    (Components|StaticMesh|SetStaticMesh (Variables|Default|GetStaticMesh5) (LocalVariables|GetcurrMesh))
    (Components|StaticMesh|SetStaticMesh (Variables|Default|GetStaticMesh14) (LocalVariables|GetcurrMesh))
    (Components|StaticMesh|SetStaticMesh (Variables|Default|GetStaticMesh7) (LocalVariables|GetcurrMesh))
    (Components|StaticMesh|SetStaticMesh (Variables|Default|GetStaticMesh8) (LocalVariables|GetcurrMesh))
    (Components|StaticMesh|SetStaticMesh (Variables|Default|GetStaticMesh13) (LocalVariables|GetcurrMesh))
    (Components|StaticMesh|SetStaticMesh (Variables|Default|GetStaticMesh6) (LocalVariables|GetcurrMesh))
    (Components|StaticMesh|SetStaticMesh (Variables|Default|GetStaticMesh11) (LocalVariables|GetcurrMesh))
    (Components|StaticMesh|SetStaticMesh (Variables|Default|GetStaticMesh12) (LocalVariables|GetcurrMesh))
    (Components|StaticMesh|SetStaticMesh (Variables|Default|GetStaticMesh3) (LocalVariables|GetcurrMesh))
    (Components|StaticMesh|SetStaticMesh (Variables|Default|GetStaticMesh10) (LocalVariables|GetcurrMesh))
    (else
      ;[1 1 1] If railroad
      (if (== (LocalVariables|GetcurrMesh) "/Game/StarterContent/Other/railroad.railroad")
        (goto _label)
        (elif (== _output_get "/Game/StarterContent/River/waterbrightBase.waterbrightBase")
          ;[1 1 1] Set water tiles
          (LocalVariables|SetcurrMesh "/Game/StarterContent/River/waterdarkBase.waterdarkBase")
          (Components|StaticMesh|SetStaticMesh (Variables|Default|GetStaticMesh) (LocalVariables|GetcurrMesh))
          (LocalVariables|SetcurrMesh "/Game/StarterContent/River/waterbrightTop.waterbrightTop")
          (Components|StaticMesh|SetStaticMesh (Variables|Default|GetStaticMesh1) (LocalVariables|GetcurrMesh))
          (LocalVariables|SetcurrMesh "/Game/StarterContent/River/waterbrightBase.waterbrightBase")
          (Components|StaticMesh|SetStaticMesh (Variables|Default|GetStaticMesh2) (LocalVariables|GetcurrMesh))
          (Components|StaticMesh|SetStaticMesh (Variables|Default|GetStaticMesh3) (LocalVariables|GetcurrMesh))
          (Components|StaticMesh|SetStaticMesh (Variables|Default|GetStaticMesh4) (LocalVariables|GetcurrMesh))
          (Components|StaticMesh|SetStaticMesh (Variables|Default|GetStaticMesh5) (LocalVariables|GetcurrMesh))
          (Components|StaticMesh|SetStaticMesh (Variables|Default|GetStaticMesh6) (LocalVariables|GetcurrMesh))
          (Components|StaticMesh|SetStaticMesh (Variables|Default|GetStaticMesh7) (LocalVariables|GetcurrMesh))
          (Components|StaticMesh|SetStaticMesh (Variables|Default|GetStaticMesh8) (LocalVariables|GetcurrMesh))
          (Components|StaticMesh|SetStaticMesh (Variables|Default|GetStaticMesh9) (LocalVariables|GetcurrMesh))
          (Components|StaticMesh|SetStaticMesh (Variables|Default|GetStaticMesh10) (LocalVariables|GetcurrMesh))
          (Components|StaticMesh|SetStaticMesh (Variables|Default|GetStaticMesh11) (LocalVariables|GetcurrMesh))
          (Components|StaticMesh|SetStaticMesh (Variables|Default|GetStaticMesh12) (LocalVariables|GetcurrMesh))
          (LocalVariables|SetcurrMesh "/Game/StarterContent/River/waterbrightBottom.waterbrightBottom")
          (Components|StaticMesh|SetStaticMesh (Variables|Default|GetStaticMesh13) (LocalVariables|GetcurrMesh))
          (LocalVariables|SetcurrMesh "/Game/StarterContent/River/waterdarkBase.waterdarkBase")
          (Components|StaticMesh|SetStaticMesh (Variables|Default|GetStaticMesh14) (LocalVariables|GetcurrMesh))
          (else
            ;[1 1 1] If highway
            (if (== (LocalVariables|GetcurrMesh) "/Game/StarterContent/Other/highwayunmarked.highwayunmarked")
              ;[1 1 1] Determine if first lane
              (if (== (Variables|/Game/Blueprints/lane_spawner_bp.lane_spawner_bp_C|GetNumOfCurrentLanes _lanespawner_2) (Variables|/Game/Blueprints/lane_spawner_bp.lane_spawner_bp_C|GetNumOfCurrentLanesLargest _lanespawner_2))
                (LocalVariables|SetcurrMesh "/Game/StarterContent/Other/highwayunmarked.highwayunmarked")
                (goto _label)
                (else
                  ;[1 1 1] Set Marked Highway lane tiles
                  (Components|StaticMesh|SetStaticMesh (Variables|Default|GetStaticMesh) (LocalVariables|GetcurrMesh))
                  (LocalVariables|SetcurrMesh "/Game/StarterContent/Other/highwaymarked.highwaymarked")
                  (Components|StaticMesh|SetStaticMesh (Variables|Default|GetStaticMesh1) (LocalVariables|GetcurrMesh))
                  (LocalVariables|SetcurrMesh "/Game/StarterContent/Other/highwayunmarked.highwayunmarked")
                  (Components|StaticMesh|SetStaticMesh (Variables|Default|GetStaticMesh2) (LocalVariables|GetcurrMesh))
                  (LocalVariables|SetcurrMesh "/Game/StarterContent/Other/highwaymarked.highwaymarked")
                  (Components|StaticMesh|SetStaticMesh (Variables|Default|GetStaticMesh3) (LocalVariables|GetcurrMesh))
                  (LocalVariables|SetcurrMesh "/Game/StarterContent/Other/highwayunmarked.highwayunmarked")
                  (Components|StaticMesh|SetStaticMesh (Variables|Default|GetStaticMesh4) (LocalVariables|GetcurrMesh))
                  (LocalVariables|SetcurrMesh "/Game/StarterContent/Other/highwaymarked.highwaymarked")
                  (Components|StaticMesh|SetStaticMesh (Variables|Default|GetStaticMesh5) (LocalVariables|GetcurrMesh))
                  (LocalVariables|SetcurrMesh "/Game/StarterContent/Other/highwayunmarked.highwayunmarked")
                  (Components|StaticMesh|SetStaticMesh (Variables|Default|GetStaticMesh6) (LocalVariables|GetcurrMesh))
                  (LocalVariables|SetcurrMesh "/Game/StarterContent/Other/highwaymarked.highwaymarked")
                  (Components|StaticMesh|SetStaticMesh (Variables|Default|GetStaticMesh7) (LocalVariables|GetcurrMesh))
                  (LocalVariables|SetcurrMesh "/Game/StarterContent/Other/highwayunmarked.highwayunmarked")
                  (Components|StaticMesh|SetStaticMesh (Variables|Default|GetStaticMesh8) (LocalVariables|GetcurrMesh))
                  (LocalVariables|SetcurrMesh "/Game/StarterContent/Other/highwaymarked.highwaymarked")
                  (Components|StaticMesh|SetStaticMesh (Variables|Default|GetStaticMesh9) (LocalVariables|GetcurrMesh))
                  (LocalVariables|SetcurrMesh "/Game/StarterContent/Other/highwayunmarked.highwayunmarked")
                  (Components|StaticMesh|SetStaticMesh (Variables|Default|GetStaticMesh10) (LocalVariables|GetcurrMesh))
                  (LocalVariables|SetcurrMesh "/Game/StarterContent/Other/highwaymarked.highwaymarked")
                  (Components|StaticMesh|SetStaticMesh (Variables|Default|GetStaticMesh11) (LocalVariables|GetcurrMesh))
                  (LocalVariables|SetcurrMesh "/Game/StarterContent/Other/highwayunmarked.highwayunmarked")
                  (Components|StaticMesh|SetStaticMesh (Variables|Default|GetStaticMesh12) (LocalVariables|GetcurrMesh))
                  (LocalVariables|SetcurrMesh "/Game/StarterContent/Other/highwaymarked.highwaymarked")
                  (Components|StaticMesh|SetStaticMesh (Variables|Default|GetStaticMesh13) (LocalVariables|GetcurrMesh))
                  (LocalVariables|SetcurrMesh "/Game/StarterContent/Other/highwayunmarked.highwayunmarked")
                  (Components|StaticMesh|SetStaticMesh (Variables|Default|GetStaticMesh14) (LocalVariables|GetcurrMesh)))))))))))